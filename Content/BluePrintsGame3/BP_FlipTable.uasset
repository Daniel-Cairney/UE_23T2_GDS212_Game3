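; BP_FlipTable is an actor that scores a point and plays a bonk sound when the player pawn overlaps its Collider.
; The overlap finds every top-level VehicleUI widget and increments its Score directly, so the score lives in the UI.
; OnHitAudio then spawns the sound at the Collider's location and prints debug text.
; No flipping logic is in the graph, and NewFunction is an empty stub.
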(event `self.Collider.OnComponentBeginOverlap`
  (params (OverlappedComponent :type "PrimitiveComponent Object Reference") (OtherActor :type "Actor Object Reference") (OtherComp :type "PrimitiveComponent Object Reference") (OtherBodyIndex :type Integer) (bFromSweep :type Boolean) (SweepResult :type "HitResult Structure (by ref)"))
  (if (== OtherActor (`GameplayStatics.GetPlayerPawn` 0))
    (`|ExecutionSequence`
      (:`then_0`
        (bind _foundwidgets (`WidgetBlueprintLibrary.GetAllWidgetsOfClass` "/Game/VehicleTemplate/Blueprints/VehicleUI.VehicleUI_C"))
        (for _array_element _foundwidgets
          (set `/Game/VehicleTemplate/Blueprints/VehicleUI.Score` (+ (`/Game/VehicleTemplate/Blueprints/VehicleUI.Score` _array_element) 1) _array_element)
          (`KismetSystemLibrary.PrintString` "Added 1 to score")))
      (:`then_1`
        (`self.OnHitAudio`)))))

(event `OnHitAudio`
  (bind _returnvalue (`GameplayStatics.SpawnSoundAtLocation` "/Game/Audio/bonk-sound-effect.bonk-sound-effect" (`SceneComponent.K2_GetComponentLocation` (`self.Collider`)) (struct) 1.0 1.0 0.0 null null))
  (`AudioComponent.Play` _returnvalue 0.0)
  (`KismetSystemLibrary.PrintText` "Bonk"))

(fn `NewFunction`)

(fn `UserConstructionScript`)